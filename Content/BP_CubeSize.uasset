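; BP_CubeSize is an actor that shrinks in fixed steps when other actors overlap it.
; BeginPlay stores one tenth of the starting scale as Delta.
; Each overlap waits on a short Delay, then subtracts Delta from the current scale, so overlaps during a pending delay add no extra step.
; The shrink has no lower limit, and Tick and the construction script only call their parents.
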(event EventBeginPlay
  (|CallParentFunction)
  (Variables|Default|Setdelta (/ (Transformation|GetActorScale3D) 1e+01)))

(event Collision|EventActorBeginOverlap
  (params (OtherActor :type Actor%20Object%20Reference))
  (|CallParentFunction OtherActor)
  (Utilities|FlowControl|Delay 0.2)
  (Transformation|SetActorScale3D (- (Transformation|GetActorScale3D) (Variables|Default|Getdelta))))

(event EventTick
  (params (DeltaSeconds :type Float%20%28single-precision%29))
  (|CallParentFunction DeltaSeconds))

(fn ConstructionScript
  (|CallParentFunction))